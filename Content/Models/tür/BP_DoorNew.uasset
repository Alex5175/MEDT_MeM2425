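; BP_DoorNew is a grabbable door that swings open or closed, apparently for VR interaction.
; Each grab flips between playing and reversing the Swing timeline, which drives the Scene component's yaw through up to a quarter turn; release does nothing.
; An older hand-following approach remains disconnected: a looping timer meant to run UpdateRotation, which turns motion controller offset into clamped yaw.
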(event OnGrabbed(GrabComponent)
  (params (MotionController :type Motion%20Controller%20Component%20Object%20Reference))
  (Utilities|FlowControl|FlipFlop
    (:A
      (bind _swingtrack (Timeline|Swing Play)
        (:Update
          (Transformation|SetRelativeRotation (Variables|Default|GetScene) (Math|Rotator|MakeRotator 0.0 0.0 (* _swingtrack 9e+01)) false false))))
    (:B
      (Timeline|Swing Reverse))))

(event OnDropped(GrabComponent))

(fn ConstructionScript)

(fn UpdateRotation
  (bind _grabcomponent (Variables|Default|GetGrabComponent))
  (bind _scene (Variables|Default|GetScene))
  (bind _relativerotation (Variables|/Script/Engine.SceneComponent|GetRelativeRotation _scene))
  (Transformation|SetRelativeRotation _scene (Math|Rotator|MakeRotator (.roll _relativerotation) (.pitch _relativerotation) (Math|Float|Clamp(Float) (+ (.yaw _relativerotation) (.x (- (Variables|/Script/Engine.SceneComponent|GetRelativeLocation _grabcomponent) (.location (Math|Transform|MakeRelativeTransform (Transformation|GetWorldTransform (Variables|Default|GetMotion%20Controller)) (Transformation|GetWorldTransform _grabcomponent)))))) -9e+01 9e+01)) false false))